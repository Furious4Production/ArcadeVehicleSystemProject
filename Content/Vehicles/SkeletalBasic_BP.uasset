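; SkeletalBasic_BP is a basic vehicle Blueprint that routes player input to its movement and camera components.
; Move axes set acceleration and turning on MovementComponent, and the Drift action turns drift input on while held.
; Look axes add yaw and pitch to FrontCameraController, which also switches to the rear camera while RearCameraToggle is held.
; The construction script only calls its parent.
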(event Input|ActionEvents|InputActionDrift
  (params (Key :type Key%20Structure :default "None"))
  ;[1 0 0.4922] Basic inputs for the vehicle.
  (:Pressed
    (Class|ArcadeVehicleMovementComponent|SetDriftInput (Variables|Default|GetMovementComponent) true))
  (:Released
    (Class|ArcadeVehicleMovementComponent|SetDriftInput (Variables|Default|GetMovementComponent) false)))

(event Input|ActionEvents|InputActionRearCameraToggle
  (params (Key :type Key%20Structure :default "None"))
  (bind _frontcameracontroller (Variables|Default|GetFrontCameraController))
  ;[1 0 0.4922] Basic inputs for the vehicle.
  (:Pressed
    (Class|ArcadeVehicleCameraController|ActivateRearCamera _frontcameracontroller))
  (:Released
    (Class|ArcadeVehicleCameraController|ActivateFrontCamera _frontcameracontroller)))

(event Input|AxisEvents|InputAxisTurn
  (params (AxisValue :type Float%20%28single-precision%29))
  ;[1 0 0.4922] Basic inputs for the vehicle.
  (Class|ArcadeVehicleCameraController|AddYawInput (Variables|Default|GetFrontCameraController) AxisValue))

(event Input|AxisEvents|InputAxisLookUp
  (params (AxisValue :type Float%20%28single-precision%29))
  ;[1 0 0.4922] Basic inputs for the vehicle.
  (Class|ArcadeVehicleCameraController|AddPitchInput (Variables|Default|GetFrontCameraController) AxisValue))

(event Input|AxisEvents|InputAxisMoveForward
  (params (AxisValue :type Float%20%28single-precision%29))
  ;[1 0 0.4922] Basic inputs for the vehicle.
  (Class|ArcadeVehicleMovementComponent|SetAccelerationInput (Variables|Default|GetMovementComponent) AxisValue))

(event Input|AxisEvents|InputAxisMoveRight
  (params (AxisValue :type Float%20%28single-precision%29))
  ;[1 0 0.4922] Basic inputs for the vehicle.
  (Class|ArcadeVehicleMovementComponent|SetTurningInput (Variables|Default|GetMovementComponent) AxisValue))

(fn ConstructionScript
  (|CallParentFunction))